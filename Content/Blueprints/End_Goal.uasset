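; End-goal actor that destroys any actor overlapping it and costs the player a life.
; It finds the first Variable_Holder_Blueprint in the level on each overlap and decrements its Lives.
; When Lives reaches zero or below, it pauses the game, creates the Game_Over widget without adding it to the viewport here, and shows the mouse cursor.
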(event `self.ReceiveActorBeginOverlap`
  (params (OtherActor :type "Actor Object Reference"))
  (if (`KismetSystemLibrary.IsValid` OtherActor)
    (`self.K2_DestroyActor` OtherActor)
    (bind _outactors (`GameplayStatics.GetAllActorsOfClass` "/Game/Blueprints/Variable_Holder_Blueprint.Variable_Holder_Blueprint_C"))
    (bind _asvariable_holder_blueprint (cast `/Game/Blueprints/Variable_Holder_Blueprint` (`|GetArrayItem` _outactors)))
    (bind _output_get (set `/Game/Blueprints/Variable_Holder_Blueprint.Lives` (- (`/Game/Blueprints/Variable_Holder_Blueprint.Lives` _asvariable_holder_blueprint) 1) _asvariable_holder_blueprint))
    (if (<= _output_get 0)
      (`GameplayStatics.SetGamePaused` true)
      (`|CreateWidget` "/Game/UI/Game_Over.Game_Over_C")
      (set `PlayerController.bShowMouseCursor` true (`GameplayStatics.GetPlayerController` 0)))))

(fn `UserConstructionScript`)