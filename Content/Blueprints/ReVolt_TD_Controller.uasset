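; ReVolt tower defense controller that opens the Difficulty_Chooser widget on BeginPlay and enables mouse cursor, click, mouse-over and touch input.
; Left click and touch share one path that traces under the cursor on the Camera channel, applies a small amount of damage to the hit actor and prints its name for debugging.
; MoveToHitLocation and the construction script are empty.
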(event `self.ReceiveBeginPlay`
  (bind _returnvalue (`|CreateWidget` "/Game/UI/Difficulty_Chooser.Difficulty_Chooser_C"))
  (`UserWidget.AddToViewport` _returnvalue 0)
  (set `self.bShowMouseCursor` true)
  (set `self.bEnableClickEvents` true)
  (set `self.bEnableMouseOverEvents` true)
  (set `self.bEnableTouchEvents` true)
  (set `self.bEnableTouchEvents` true))

(event `InputTouch`
  (params (Location :type "Vector Structure") (FingerIndex :type "ETouchIndex Enum"))
  (:`Pressed`
    (bind _output_get (set `self.Mouse_Hit_actor` (`.HitActor` (`GameplayStatics.BreakHitResult` (`self.GetHitResultUnderCursorByChannel` "TraceTypeQuery2"))) :!label _label))
    (`GameplayStatics.ApplyDamage` _output_get 0.05 null null "/Script/Engine.DamageType")
    (`KismetSystemLibrary.PrintString` (`KismetStringLibrary.Concat_StrStr` "Attempting to damage " (`KismetSystemLibrary.GetDisplayName` _output_get)))))

(event `Key|LeftMouseButton`
  (params (Key :type "Key Structure"))
  (:`Pressed`
    (goto _label)))

(fn `MoveToHitLocation`
  (params (NewParam :type "HitResult Structure")))

(fn `UserConstructionScript`)