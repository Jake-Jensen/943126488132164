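; BasicTurret is a turret actor that turns to face a Basic_Enemy_1 and damages it.
; Getnearest returns the Nearest variable, set to the last enemy within the ClosestDist–MinDist band rather than the true closest.
; Tick yaws toward that target, then uses Delays to apply damage and show a brief explosion.
; A parallel delayed branch destroys all Basic_Enemy_1 actors if Hidden is set.
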(event `self.ReceiveTick`
  (params (DeltaSeconds :type "Float (single-precision)"))
  ;[1 1 1] targetting
  (`|ExecutionSequence`
    (:`then_0`
      (bind _nearest (`self.Get-nearest`))
      (`/Engine/EditorBlueprintResources/StandardMacros.IsValid` _nearest
        (:`Is Valid`
          (bind _returnvalue (`self.K2_GetActorLocation` _nearest))
          (`SceneComponent.K2_SetWorldRotation` (`self.RootComponent`) (`KismetMathLibrary.MakeRotator` 0.0 0.0 (- (.yaw (`KismetMathLibrary.FindLookAtRotation` (`self.K2_GetActorLocation` self) _returnvalue)) 90.0)) false false)
          (`KismetSystemLibrary.Delay` 1.5)
          (`GameplayStatics.ApplyDamage` _nearest (`self.Damage`) null null "/Script/Engine.DamageType")
          (bind _returnvalue_2 (`GameplayStatics.SpawnEmitterAtLocation` "/Game/StarterContent/Particles/P_Explosion.P_Explosion" _returnvalue (struct) (1.0 1.0 1.0) false))
          (`KismetSystemLibrary.Delay` 0.3)
          (`ActorComponent.K2_DestroyComponent` _returnvalue_2))))
    (:`then_1`
      (`KismetSystemLibrary.Delay` 7.0)
      (bind _outactors (`GameplayStatics.GetAllActorsOfClass` "/Game/Blueprints/Basic_Enemy_1.Basic_Enemy_1_C"))
      (for _array_element _outactors
        (if (`self.bHidden`)
          (if (`KismetSystemLibrary.IsValid` _array_element)
            (`self.K2_DestroyActor` _array_element)))))))

(fn `Get-nearest`
  (returns (Nearest :type "/Game/Blueprints/Basic_Enemy_1 Object Reference"))
  (bind _outactors (`GameplayStatics.GetAllActorsOfClass` "/Game/Blueprints/Basic_Enemy_1.Basic_Enemy_1_C"))
  (for _array_element _outactors
    (bind _returnvalue (`self.GetDistanceTo` _array_element))
    (if (and (< _returnvalue (`self.Min_Dist`)) (> _returnvalue (`self.Closest_Dist`)))
      (set `self.Nearest` _array_element)))
  (return (`self.Nearest`)))

(fn `UserConstructionScript`)