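; Basic enemy pawn that travels to the End_Plate_Blueprint actor and rewards money when killed.
; On BeginPlay it reads max HP and difficulty from the shared Variable_Holder_Blueprint, sets its movement speed by difficulty, then scales itself and starts AIMoveTo.
; AnyDamage subtracts health; at zero it spawns an explosion, destroys itself and updates the holder's death count and money.
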(event `self.ReceiveAnyDamage`
  (params (Damage :type "Float (single-precision)") (DamageType :type "DamageType Object Reference") (InstigatedBy :type "Controller Object Reference") (DamageCauser :type "Actor Object Reference"))
  (bind _current_hp (`self.Current-hp`))
  (set `self.Current-hp` (- _current_hp Damage))
  (if (not (> _current_hp 0.0))
    (`GameplayStatics.SpawnEmitterAtLocation` "/Game/StarterContent/Particles/P_Explosion.P_Explosion" (`self.K2_GetActorLocation`))
    (if (not (`KismetSystemLibrary.IsValid` self))
      (`self.K2_SetActorLocation` (0.0 0.0 -999999.0) false true)
      (`KismetSystemLibrary.Delay` 5.0))
    (`self.K2_DestroyActor`)
    (bind _outactors (`GameplayStatics.GetAllActorsOfClass` "/Game/Blueprints/Variable_Holder_Blueprint.Variable_Holder_Blueprint_C"))
    (bind _asvariable_holder_blueprint (cast `/Game/Blueprints/Variable_Holder_Blueprint` (`|GetArrayItem` _outactors)))
    (set `/Game/Blueprints/Variable_Holder_Blueprint.Number_Of_Dead` (+ (`/Game/Blueprints/Variable_Holder_Blueprint.Number_Of_Dead` _asvariable_holder_blueprint) 1) _asvariable_holder_blueprint)
    (set `/Game/Blueprints/Variable_Holder_Blueprint.Money` (+ (`/Game/Blueprints/Variable_Holder_Blueprint.Money` _asvariable_holder_blueprint) (`/Game/Blueprints/Variable_Holder_Blueprint.Money_To_Add` _asvariable_holder_blueprint)) _asvariable_holder_blueprint)))

(event `self.ReceiveBeginPlay`
  (bind _floatingpawnmovement (`self.FloatingPawnMovement`))
  (bind _outactors (`GameplayStatics.GetAllActorsOfClass` "/Game/Blueprints/Variable_Holder_Blueprint.Variable_Holder_Blueprint_C"))
  (bind _asvariable_holder_blueprint (cast `/Game/Blueprints/Variable_Holder_Blueprint` (`|GetArrayItem` _outactors)))
  (set `self.Max-HP` (`/Game/Blueprints/Variable_Holder_Blueprint.Maximum_HP` _asvariable_holder_blueprint))
  (set `self.Current-hp` (`self.Max-HP`))
  (switch `int` (`/Game/Blueprints/Variable_Holder_Blueprint.Difficulty` _asvariable_holder_blueprint)
    (:`0`
      (set `FloatingPawnMovement.MaxSpeed` 80.0 _floatingpawnmovement))
    (:`1`
      (set `FloatingPawnMovement.MaxSpeed` 120.0 _floatingpawnmovement))
    (:`2`
      (set `FloatingPawnMovement.MaxSpeed` 300.0 _floatingpawnmovement))
    (:`3`
      (set `FloatingPawnMovement.MaxSpeed` 750.0 _floatingpawnmovement)))
  (bind _outactors_2 (`GameplayStatics.GetAllActorsOfClass` "/Game/Blueprints/End_Plate_Blueprint.End_Plate_Blueprint_C"))
  (bind _asend_plate_blueprint (cast `/Game/Blueprints/End_Plate_Blueprint` (`|GetArrayItem` _outactors_2)))
  (`self.SetActorEnableCollision` true)
  (`self.SetActorScale3D` (0.5 0.5 0.5))
  (`|AIMoveTo` self (0.0 0.0 0.0) _asend_plate_blueprint
    (:`then`
      (`KismetSystemLibrary.Delay` 0.7)
      (`KismetSystemLibrary.PrintString` (`KismetStringLibrary.Conv_DoubleToString` (`self.Max-HP`))))))

(event `self.ReceivePossessed`
  (params (NewController :type "Controller Object Reference")))

(fn `UserConstructionScript`)