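; Player camera and controller logic for the ReVolt tower defense game, handling setup, movement and tower placement.
; BeginPlay initializes money, lives and help text and pauses behind the difficulty chooser; Add_Main_Hud creates the HUD and sets MaxLoop by difficulty.
; Axis input pans along X/Y; Space or mouse spawns the HUD-selected tower on a pad and deducts money.
; Easy enemy spawning fires a "ce" console command; other difficulty spawn events are empty.
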(event `self.ReceiveBeginPlay`
  ;[1 1 1] Main Variables
  (set `PlayerController.bEnableTouchEvents` true (`GameplayStatics.GetPlayerController` 0))
  (bind _output_get (set `self.Start_Location` (`self.K2_GetActorLocation` (`GameplayStatics.GetPlayerPawn` 0))))
  (set `self.Current_Location` _output_get)
  (set `self.Movement_Sensitivity` 7.0)
  (set `self.Difficulty` "NOT_SELECTED")
  (bind _returnvalue (`|CreateWidget` "/Game/UI/Difficulty_Chooser.Difficulty_Chooser_C"))
  (`UserWidget.AddToViewport` _returnvalue 0)
  (`GameplayStatics.SetGamePaused` true)
  (set `self.Money` 100.0)
  (set `self.Lives` 100)
  (set `self.Help_Box_Text` "Welcome to ReVolt! \nTo begin, select a tower then move to a pad.  \nOnce there, click your mouse or click the space key to build a tower."))

(event `Add_Main_Hud`
  ;[1 1 1] Main Variables
  (`KismetSystemLibrary.Delay` 0.2)
  (bind _returnvalue (`|CreateWidget` "/Game/UI/Main_Hud.Main_Hud_C"))
  (`WidgetBlueprintLibrary.SetInputMode_GameOnly` (`GameplayStatics.GetPlayerController` 0))
  (bind _output_get (set `self.Main_Hud_Cast_For_Tick` _returnvalue))
  (`UserWidget.AddToViewport` _returnvalue 0)
  (`UserWidget.AddToViewport` _output_get 0)
  (switch `string` (`self.Difficulty`)
    (:`Easy`
      (set `self.Max_Loop` 50))
    (:`Medium`
      (set `self.Max_Loop` 100))
    (:`hard`
      (set `self.Max_Loop` 150))
    (:`nightmare`
      (set `self.Max_Loop` 200))))

(event `InputAxis|MoveForward`
  (params (AxisValue :type "Float (single-precision)"))
  (bind _movement_sensitivity (`self.Movement_Sensitivity`))
  (bind (_current_location_x _current_location_y _current_location_z) (`KismetMathLibrary.BreakVector` (`self.Current_Location`)))
  (bind (_current_location_x_2 _current_location_y_2 _current_location_z_2) (`KismetMathLibrary.BreakVector` (`self.Current_Location`)))
  (bind _returnvalue (`KismetMathLibrary.MakeVector` (+ _current_location_x _movement_sensitivity) _current_location_y _current_location_z))
  (bind _returnvalue_2 (`KismetMathLibrary.MakeVector` (- _current_location_x_2 _movement_sensitivity) _current_location_y_2 _current_location_z_2))
  ;[1 1 1] Camera Movement
  (if (>= AxisValue 0.9)
    (`self.K2_SetActorLocation` _returnvalue)
    (set `self.Current_Location` _returnvalue)
    (elif (<= AxisValue -0.9)
      (`self.K2_SetActorLocation` _returnvalue_2)
      (set `self.Current_Location` _returnvalue_2))))

(event `InputAxis|MoveRight`
  (params (AxisValue :type "Float (single-precision)"))
  (bind (_current_location_x _current_location_y _current_location_z) (`KismetMathLibrary.BreakVector` (`self.Current_Location`)))
  (bind (_current_location_x_2 _current_location_y_2 _current_location_z_2) (`KismetMathLibrary.BreakVector` (`self.Current_Location`)))
  (bind _movement_sensitivity (`self.Movement_Sensitivity`))
  (bind _returnvalue (`KismetMathLibrary.MakeVector` _current_location_x (- _current_location_y _movement_sensitivity) _current_location_z))
  (bind _returnvalue_2 (`KismetMathLibrary.MakeVector` _current_location_x_2 (+ _current_location_y_2 _movement_sensitivity) _current_location_z_2))
  ;[1 1 1] Camera Movement
  (if (>= AxisValue 0.9)
    (`self.K2_SetActorLocation` _returnvalue_2)
    (set `self.Current_Location` _returnvalue_2)
    (elif (<= AxisValue -0.9)
      (`self.K2_SetActorLocation` _returnvalue)
      (set `self.Current_Location` _returnvalue))))

(event `Spawn_Easy_terra`
  ;[1 1 1] Enemy spawning
  (`KismetSystemLibrary.ExecuteConsoleCommand` "ce Spawn_Easy" null))

(event `Spawn_Med_Terra`
  ;[1 1 1] Enemy spawning
)

(event `Spawn_Hard_Terra`
  ;[1 1 1] Enemy spawning
)

(event `Spawn_Nightmare_Terra`
  ;[1 1 1] Enemy spawning
)

(event `Key|SpaceBar`
  (params (Key :type "Key Structure"))
  ;[1 1 1] Handle tower spawning
  (:`Pressed`
    (bind _foundwidgets (`WidgetBlueprintLibrary.GetAllWidgetsOfClass` "/Game/UI/Main_Hud.Main_Hud_C" :!label _label))
    (bind _asmain_hud (cast `/Game/UI/Main_Hud` (`|GetArrayItem` _foundwidgets)))
    (if (`/Game/UI/Main_Hud.On_Spawn_Pad` _asmain_hud)
      (if (`/Game/UI/Main_Hud.Holding_Basic_Tower` _asmain_hud)
        (bind _returnvalue (`|SpawnActorFromClass` "/Game/Blueprints/BasicTurret.BasicTurret_C" (`KismetMathLibrary.Conv_VectorToTransform` (`/Game/UI/Main_Hud.Spawn_Pad_Location` _asmain_hud)) "AdjustIfPossibleButDontSpawnIfColliding" "OverrideRootScale" null null))
        (`/Engine/EditorBlueprintResources/StandardMacros.IsValid` _returnvalue
          (:`Is Valid`
            (`/Game/UI/Main_Hud.Subtract_Money_Basic_Tower` _asmain_hud)))
        (else
          (`KismetSystemLibrary.PrintText` "Skipping basic tower")
          (if (`/Game/UI/Main_Hud.Holding_Magic_Tower` _asmain_hud)
            (bind _returnvalue_2 (`|SpawnActorFromClass` "/Game/Blueprints/Tower_Magoc_5.Tower_Magoc_5_C" (`KismetMathLibrary.Conv_VectorToTransform` (`/Game/UI/Main_Hud.Spawn_Pad_Location` _asmain_hud)) "AdjustIfPossibleButDontSpawnIfColliding" "OverrideRootScale" null null))
            (`/Engine/EditorBlueprintResources/StandardMacros.IsValid` _returnvalue_2
              (:`Is Valid`
                (`self.SetActorScale3D` _returnvalue_2 (0.2 0.2 0.2))
                (`/Game/UI/Main_Hud.Subtract_Money_Magic_Tower` _asmain_hud)))
            (else
              (`KismetSystemLibrary.PrintText` "Skipping magic tower")))))
      (else
        (`KismetSystemLibrary.PrintText` "Ignoring input")))))

(event `InputAction|Mouse_Action`
  (params (Key :type "Key Structure"))
  ;[1 1 1] Handle tower spawning
  (:`Pressed`
    (goto _label)))

(fn `UserConstructionScript`)