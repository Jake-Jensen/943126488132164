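; Spawn pad actor that tells the Main_Hud widget when something is standing on it.
; On begin overlap it finds the HUD through a widget class search, writes its own location to SpawnPadLocation, sets OnSpawnPad and caches a HUD reference.
; End overlap clears the flag.
; Neither event filters the overlapping actor, so any overlap updates the HUD.
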(event `self.ReceiveActorBeginOverlap`
  (params (OtherActor :type "Actor Object Reference"))
  (bind _foundwidgets (`WidgetBlueprintLibrary.GetAllWidgetsOfClass` "/Game/UI/Main_Hud.Main_Hud_C" false))
  (bind _asmain_hud (cast `/Game/UI/Main_Hud` (`|GetArrayItem` _foundwidgets)))
  (set `/Game/UI/Main_Hud.Spawn_Pad_Location` (`self.K2_GetActorLocation`) _asmain_hud)
  (set `/Game/UI/Main_Hud.On_Spawn_Pad` true _asmain_hud)
  (bind _foundwidgets_2 (`WidgetBlueprintLibrary.GetAllWidgetsOfClass` "/Game/UI/Main_Hud.Main_Hud_C"))
  (bind _asmain_hud_2 (cast `/Game/UI/Main_Hud` (`|GetArrayItem` _foundwidgets_2)))
  (set `self.Main_Hud_Cast` _asmain_hud_2))

(event `self.ReceiveActorEndOverlap`
  (params (OtherActor :type "Actor Object Reference"))
  (bind _foundwidgets (`WidgetBlueprintLibrary.GetAllWidgetsOfClass` "/Game/UI/Main_Hud.Main_Hud_C" false))
  (bind _asmain_hud (cast `/Game/UI/Main_Hud` (`|GetArrayItem` _foundwidgets)))
  (set `/Game/UI/Main_Hud.On_Spawn_Pad` false _asmain_hud))

(fn `UserConstructionScript`)