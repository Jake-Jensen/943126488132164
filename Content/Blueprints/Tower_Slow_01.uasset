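; Tower actor that turns to face an enemy in range and deals radial damage around it; no slowing logic is present.
; GetNearest returns the last Basic_Enemy_1 between ClosestDist and MinDist, not necessarily the nearest.
; Tick rotates yaw toward that target, then a one-second Delay gates the damage, which ignores all 16x1 actors.
; An explosion particle branch is disconnected and never runs.
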(event `self.ReceiveBeginPlay`
  ;[1 1 1] targetting
)

(event `self.ReceiveTick`
  (params (DeltaSeconds :type "Float (single-precision)"))
  ;[1 1 1] targetting
  (bind _nearest (`self.Get-Nearest`))
  (`/Engine/EditorBlueprintResources/StandardMacros.IsValid` _nearest
    (:`Is Valid`
      (bind _returnvalue (`self.K2_GetActorLocation` _nearest))
      (`SceneComponent.K2_SetWorldRotation` (`self.RootComponent`) (`KismetMathLibrary.MakeRotator` 0.0 0.0 (+ (.yaw (`KismetMathLibrary.FindLookAtRotation` (`self.K2_GetActorLocation` self) _returnvalue)) -180.0)) false false)
      (`KismetSystemLibrary.Delay` 1.0)
      (bind _outactors (`GameplayStatics.GetAllActorsOfClass` "/Game/Blueprints/Tiles/16x1.16x1_C"))
      (`GameplayStatics.ApplyRadialDamage` (`self.Damage`) _returnvalue 200.0 "/Script/Engine.DamageType" _outactors null null))))

(fn `Get-Nearest`
  (returns (Nearest :type "/Game/Blueprints/Basic_Enemy_1 Object Reference"))
  (bind _outactors (`GameplayStatics.GetAllActorsOfClass` "/Game/Blueprints/Basic_Enemy_1.Basic_Enemy_1_C"))
  (for _array_element _outactors
    (`/Engine/EditorBlueprintResources/StandardMacros.IsValid` _array_element
      (:`Is Valid`
        (bind _returnvalue (`self.GetDistanceTo` _array_element))
        (if (and (< _returnvalue (`self.Min_Dist`)) (> _returnvalue (`self.Closest_Dist`)))
          (set `self.NewVar_0` _array_element)))
      (:`Is Not Valid`
        (`KismetSystemLibrary.PrintText` "Target is invalid!"))))
  (return (`self.NewVar_0`)))

(fn `UserConstructionScript`)