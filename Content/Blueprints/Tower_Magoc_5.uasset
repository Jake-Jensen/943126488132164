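; Tower Blueprint that turns to face an enemy in range, damages it and plays an explosion.
; GetNearest scans all Basic_Enemy_1 actors and returns the last one between the ClosestDist and MinDist bounds, not necessarily the nearest.
; Tick updates yaw toward that target, with a Delay pacing ApplyDamage.
; A scaled-down explosion emitter spawns at the target if it remains valid, and is destroyed after another short delay.
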(event `self.ReceiveBeginPlay`
  ;[1 1 1] targetting
)

(event `self.ReceiveTick`
  (params (DeltaSeconds :type "Float (single-precision)"))
  ;[1 1 1] targetting
  (bind _nearest (`self.Get-Nearest`))
  (`/Engine/EditorBlueprintResources/StandardMacros.IsValid` _nearest
    (:`Is Valid`
      (bind _returnvalue (`self.K2_GetActorLocation` _nearest))
      (`SceneComponent.K2_SetWorldRotation` (`self.RootComponent`) (`KismetMathLibrary.MakeRotator` 0.0 0.0 (+ (.yaw (`KismetMathLibrary.FindLookAtRotation` (`self.K2_GetActorLocation` self) _returnvalue)) -180.0)) false false)
      (`KismetSystemLibrary.Delay` 0.25)
      (`GameplayStatics.ApplyDamage` _nearest (`self.Damage`) null null "/Script/Engine.DamageType")
      (`/Engine/EditorBlueprintResources/StandardMacros.IsValid` _nearest
        (:`Is Valid`
          (if (`AIBlueprintHelperLibrary.IsValidAILocation` _returnvalue)
            (bind _returnvalue_2 (`GameplayStatics.SpawnEmitterAtLocation` "/Game/StarterContent/Particles/P_Explosion.P_Explosion" _returnvalue (struct) (0.3 0.3 0.3)))
            (`KismetSystemLibrary.Delay` 0.3)
            (`ActorComponent.K2_DestroyComponent` _returnvalue_2)))))))

(fn `Get-Nearest`
  (returns (Nearest :type "/Game/Blueprints/Basic_Enemy_1 Object Reference"))
  (bind _outactors (`GameplayStatics.GetAllActorsOfClass` "/Game/Blueprints/Basic_Enemy_1.Basic_Enemy_1_C"))
  (for _array_element _outactors
    (`/Engine/EditorBlueprintResources/StandardMacros.IsValid` _array_element
      (:`Is Valid`
        (bind _returnvalue (`self.GetDistanceTo` _array_element))
        (if (and (< _returnvalue (`self.Min_Dist`)) (> _returnvalue (`self.Closest_Dist`)))
          (set `self.NewVar_0` _array_element)))
      (:`Is Not Valid`
        (`KismetSystemLibrary.PrintText` "Target is invalid!"))))
  (return (`self.NewVar_0`)))

(fn `UserConstructionScript`)